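; BP_Spawner is a spawner actor that creates a batch of BP_Ball actors at random points inside its Box volume.
; The DoSpawn event runs a while loop on Count, printing each index and spawning balls with the spawner's rotation.
; Count resets to zero after each batch so the event can run again, though nothing in this Blueprint calls it.
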(event Custom|DoSpawn
  (while (< (Variables|Default|Getcount) 4)
    (Development|PrintString (Utilities|String|Append "Index : " (Utilities|String|ToString(Integer) (Variables|Default|Getcount))) true true "(R=0.000000,G=0.660000,B=1.000000,A=1.000000)" 25.0)
    (Math|Integer|IncrementInt (Variables|Default|Getcount)
      (:%20%20
        (Game|SpawnActorfromClass "/Game/MyContents/BP_Ball.BP_Ball_C" (Math|Transform|MakeTransform (Math|Random|RandomPointinBoundingBox (Transformation|GetActorLocation) (Components|Box|GetScaledBoxExtent (Variables|Default|GetBox))) (Transformation|GetActorRotation) "1.000000,1.000000,1.000000") "Undefined" "MultiplyWithRoot" 0 0))))
  (Variables|Default|Setcount 0))

(fn ConstructionScript)