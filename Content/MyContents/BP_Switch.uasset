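; BP_Switch is a pressure-plate style switch actor that turns linked moving objects on and off while something overlaps its Cube.
; Begin overlap sets IsPlay to true on the MoveActor, MoveRect and MoveStair references, and end overlap sets it back to false.
; Each reference is validity-checked, printing "None" when unset, and any overlapping actor triggers it without filtering.
; Debug prints of overlap details are present but disconnected.
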(event OnComponentBeginOverlap(Cube)
  (params (OverlappedComponent :type Primitive%20Component%20Object%20Reference) (OtherActor :type Actor%20Object%20Reference) (OtherComp :type Primitive%20Component%20Object%20Reference) (OtherBodyIndex :type Integer) (bFromSweep :type Boolean) (SweepResult :type Hit%20Result%20Structure%20%28by%20ref%29))
  (bind _moveactor (Variables|Default|GetMoveActor))
  (bind _moverect (Variables|Default|GetMoveRect))
  (bind _movestair (Variables|Default|GetMoveStair))
  (Utilities|FlowControl|Sequence
    (:then_0
      (Utilities|IsValid _moveactor
        (:Is%20Valid
          (Variables|/Game/MyContents/BP_MoveActor.BP_MoveActor_C|SetIsPlay _moveactor true))
        (:Is%20Not%20Valid
          (Development|PrintString "None" true true "(R=1.000000,G=0.000979,B=0.007186,A=1.000000)" 5.0))))
    (:then_1
      (Utilities|IsValid _moverect
        (:Is%20Valid
          (Variables|/Game/MyContents/BP_MoveRect.BP_MoveRect_C|SetIsPlay _moverect true))
        (:Is%20Not%20Valid
          (Development|PrintString "None" true true "(R=1.000000,G=0.000979,B=0.007186,A=1.000000)" 5.0))))
    (:then_2
      (Utilities|IsValid _movestair
        (:Is%20Valid
          (Variables|/Game/MyContents/BP_MoveStair.BP_MoveStair_C|SetIsPlay _movestair true))
        (:Is%20Not%20Valid
          (Development|PrintString "None" true true "(R=1.000000,G=0.000979,B=0.007186,A=1.000000)" 5.0))))))

(event OnComponentEndOverlap(Cube)
  (params (OverlappedComponent :type Primitive%20Component%20Object%20Reference) (OtherActor :type Actor%20Object%20Reference) (OtherComp :type Primitive%20Component%20Object%20Reference) (OtherBodyIndex :type Integer))
  (bind _moveactor (Variables|Default|GetMoveActor))
  (bind _moverect (Variables|Default|GetMoveRect))
  (bind _movestair (Variables|Default|GetMoveStair))
  (Utilities|FlowControl|Sequence
    (:then_0
      (Utilities|IsValid _moveactor
        (:Is%20Valid
          (Variables|/Game/MyContents/BP_MoveActor.BP_MoveActor_C|SetIsPlay _moveactor false))
        (:Is%20Not%20Valid
          (Development|PrintString "None" true true "(R=1.000000,G=0.000979,B=0.007186,A=1.000000)" 5.0))))
    (:then_1
      (Utilities|IsValid _moverect
        (:Is%20Valid
          (Variables|/Game/MyContents/BP_MoveRect.BP_MoveRect_C|SetIsPlay _moverect false))
        (:Is%20Not%20Valid
          (Development|PrintString "None" true true "(R=1.000000,G=0.000979,B=0.007186,A=1.000000)" 5.0))))
    (:then_2
      (Utilities|IsValid _movestair
        (:Is%20Valid
          (Variables|/Game/MyContents/BP_MoveStair.BP_MoveStair_C|SetIsPlay _movestair false))
        (:Is%20Not%20Valid
          (Development|PrintString "None" true true "(R=1.000000,G=0.000979,B=0.007186,A=1.000000)" 5.0))))))

(fn ConstructionScript)