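; BP_MoveActor is an actor that moves its static mesh in an endless staircase, alternating rightward along X and upward along Z.
; Tick adds MoveSpeed to the active axis and sets relative location, so speed depends on frame rate.
; On reaching the active axis goal, it advances that goal by its move distance and flips IsMoveRight.
; An unconnected alternative that switches axes by counting ticks remains in the graph.
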(event EventTick
  (params (DeltaSeconds :type Float%20%28single-precision%29))
  (bind _move_speed (Variables|Default|GetMove_Speed))
  ;[0.15 0.15 0.15 0.5] 다음 목표 거리 설정하면서 움직이기
  (if (Variables|Default|GetIsMoveRight)
    ;;[0.15 0.15 0.15 0.5] 오른쪽 이동
    (bind _output_get (Variables|Default|SetLocation_X (+ (Variables|Default|GetLocation_X) _move_speed)))
    (Transformation|SetRelativeLocation (Variables|Default|GetStaticMesh) (Math|Vector|MakeVector _output_get 0.0 (stale _output_get_2)) false false)
    (if (>= (Variables|Default|GetLocation_X) (Variables|Default|GetNextGoal_X))
      (Variables|Default|SetIsMoveRight false)
      (Variables|Default|SetNextGoal_X (+ (Variables|Default|GetNextGoal_X) (Variables|Default|GetMoveDistance_X))))
    (else
      ;;[0.15 0.15 0.15 0.5] 위쪽 이동
      (bind _output_get_2 (Variables|Default|SetLocation_Z (+ (Variables|Default|GetLocation_Z) _move_speed)))
      (Transformation|SetRelativeLocation (Variables|Default|GetStaticMesh) (Math|Vector|MakeVector (Variables|Default|GetLocation_X) 0.0 _output_get_2) false false)
      (if (>= (Variables|Default|GetLocation_Z) (Variables|Default|GetNextGoal_Z))
        (Variables|Default|SetIsMoveRight true)
        (Variables|Default|SetNextGoal_Z (+ (Variables|Default|GetNextGoal_Z) (Variables|Default|GetMoveDistance_Z)))))))

(event EventBeginPlay
  (Variables|Default|SetNextGoal_X (Variables|Default|GetMoveDistance_X))
  (Variables|Default|SetNextGoal_Z (Variables|Default|GetMoveDistance_Z)))

(fn ConstructionScript)