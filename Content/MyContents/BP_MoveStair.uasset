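; BP_MoveStair is a moving stair actor whose static mesh loops along a path shaped like an Enter key in the local X-Z plane.
; While IsPlay is set, Tick runs an enum state machine: right, up, then alternating left and down in two steps back to the start.
; Each state moves the mesh's relative location by MoveSpeed per frame, unscaled by delta time, switching at full, half or zero travel distance.
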(event EventTick
  (params (DeltaSeconds :type Float%20%28single-precision%29))
  (if (Variables|Default|GetIsPlay)
    (switch Utilities|FlowControl|Switch|SwitchonEN_MoveTypeStair (Variables|Default|GetEnSwitch)
      (:NewEnumerator0
        ;[0.15 0.15 0.15 0.5] 엔터키 모양으로 돌아가는
        ;;[0.15 0.15 0.15 0.5] 오른쪽
        (bind _output_get (Variables|Default|SetLocation_X (+ (Variables|Default|GetLocation_X) (Variables|Default|GetMove_Speed))))
        (Transformation|SetRelativeLocation (Variables|Default|GetStaticMesh) (Math|Vector|MakeVector _output_get 0.0 (Variables|Default|GetLocation_Z)) false false)
        (if (>= (Variables|Default|GetLocation_X) (Variables|Default|GetMoveDistance_X))
          (Variables|Default|SetEnSwitch "NewEnumerator1")))
      (:NewEnumerator1
        ;;[0.15 0.15 0.15 0.5] 위쪽
        (bind _output_get_2 (Variables|Default|SetLocation_Z (+ (Variables|Default|GetLocation_Z) (Variables|Default|GetMove_Speed))))
        (Transformation|SetRelativeLocation (Variables|Default|GetStaticMesh) (Math|Vector|MakeVector (Variables|Default|GetLocation_X) 0.0 _output_get_2) false false)
        (if (>= (Variables|Default|GetLocation_Z) (Variables|Default|GetMoveDistance_Z))
          (Variables|Default|SetEnSwitch "NewEnumerator2")))
      (:NewEnumerator2
        ;;[0.15 0.15 0.15 0.5] 왼쪽A
        (bind _output_get_3 (Variables|Default|SetLocation_X (- (Variables|Default|GetLocation_X) (Variables|Default|GetMove_Speed))))
        (Transformation|SetRelativeLocation (Variables|Default|GetStaticMesh) (Math|Vector|MakeVector _output_get_3 0.0 (Variables|Default|GetLocation_Z)) false false)
        (if (<= (Variables|Default|GetLocation_X) (* (Variables|Default|GetMoveDistance_X) 0.5))
          (Variables|Default|SetEnSwitch "NewEnumerator3")))
      (:NewEnumerator3
        ;;[0.15 0.15 0.15 0.5] 아래쪽A
        (bind _output_get_4 (Variables|Default|SetLocation_Z (- (Variables|Default|GetLocation_Z) (Variables|Default|GetMove_Speed))))
        (Transformation|SetRelativeLocation (Variables|Default|GetStaticMesh) (Math|Vector|MakeVector (Variables|Default|GetLocation_X) 0.0 _output_get_4) false false)
        (if (<= (Variables|Default|GetLocation_Z) (* (Variables|Default|GetMoveDistance_Z) 0.5))
          (Variables|Default|SetEnSwitch "NewEnumerator4")))
      (:NewEnumerator4
        ;;[0.15 0.15 0.15 0.5] 왼쪽B
        (bind _output_get_5 (Variables|Default|SetLocation_X (- (Variables|Default|GetLocation_X) (Variables|Default|GetMove_Speed))))
        (Transformation|SetRelativeLocation (Variables|Default|GetStaticMesh) (Math|Vector|MakeVector _output_get_5 0.0 (Variables|Default|GetLocation_Z)) false false)
        (if (<= (Variables|Default|GetLocation_X) 0.0)
          (Variables|Default|SetEnSwitch "NewEnumerator5")))
      (:NewEnumerator5
        ;;[0.15 0.15 0.15 0.5] 아래쪽B
        (bind _output_get_6 (Variables|Default|SetLocation_Z (- (Variables|Default|GetLocation_Z) (Variables|Default|GetMove_Speed))))
        (Transformation|SetRelativeLocation (Variables|Default|GetStaticMesh) (Math|Vector|MakeVector (Variables|Default|GetLocation_X) 0.0 _output_get_6) false false)
        (if (<= (Variables|Default|GetLocation_Z) 0.0)
          (Variables|Default|SetEnSwitch "NewEnumerator0"))))))

(event EventBeginPlay)

(fn ConstructionScript)